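; B_KankaYapıcı is a zone actor that turns an overlapping B_GM into a newly spawned B_Kanka.
; On overlap, it spawns the B_Kanka at the transform of the PlayerStart found by class lookup.
; The B_GM's owning B_GMKontroller then possesses the new actor, and the B_GM is destroyed.
; The controller cast follows the spawn, so a failed cast leaves both actors in the world.
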(event `self.ReceiveActorBeginOverlap`
  (params (OtherActor :type "Actor Object Reference"))
  (bind _asb_gm (cast `/Game/SICIRT/Karakter/GM/B_GM` OtherActor))
  (bind _returnvalue (`self.Get Player Start Transform`))
  (bind _returnvalue_2 (`|SpawnActorFromClass` "/Game/SICIRT/Karakter/Kanka/B_Kanka.B_Kanka_C" _returnvalue "Undefined" "OverrideRootScale" null null))
  (bind _asb_gmkontroller (cast `/Game/SICIRT/Karakter/GM/B_GMKontroller` (`self.GetOwner` _asb_gm)))
  (`Controller.Possess` _asb_gmkontroller _returnvalue_2)
  (`self.K2_DestroyActor` _asb_gm))

(fn `Get Player Start Transform`
  (returns (ReturnValue :type "Transform Structure (by ref)"))
  (bind _returnvalue (`GameplayStatics.GetActorOfClass` "/Script/Engine.PlayerStart"))
  (return (`self.GetTransform` _returnvalue)))

(fn `UserConstructionScript`)