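; Horror event trigger box that fires events once the player has looked or focused on it for a set duration.
; Externally called Looking and Focusing events advance separate counters in fixed steps, run HorrorEventCheck at their thresholds and reset.
; Construction applies horror event defaults and the box extent.
; Save events use the player's HESaveGameComponent cache and restore both counters, though the node packing them in MakeAssetSave is unused.
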(event `Looking`
  ;[1 1 1] Looking Settings
  (bind _output_get (set `self.LookingCounter` (+ (`self.LookingCounter`) 0.1)))
  (if (>= _output_get (`self.LookingDuration (Sec)`))
    (set `self.LookingCounter` 0.0)
    (`self.HorrorEventCheck` "NewEnumerator47")))

(event `ResetLooking`
  ;[1 1 1] Looking Settings
  (set `self.LookingCounter` 0.0))

(event `Focusing`
  ;[1 1 1] Focus Settings
  (bind _output_get (set `self.FocusingCounter` (+ (`self.FocusingCounter`) 0.1)))
  (if (>= _output_get (`self.FocusDuration (Sec)`))
    (set `self.FocusingCounter` 0.0)
    (`self.HorrorEventCheck` "NewEnumerator46")))

(event `ResetFocusing`
  ;[1 1 1] Focus Settings
  (set `self.FocusingCounter` 0.0))

(event `/Game/HorrorEngine/Blueprints/Core/HorrorEngineInterface.CollectSaveData`
  ;[0 1 0.5572] Save Settings
  (bind _asmaster (`/Game/HorrorEngine/Blueprints/Core/HorrorEngineFunctions.GetPlayer`))
  (`KismetArrayLibrary.Array_Add` (`/Game/HorrorEngine/Blueprints/Core/HE_SaveGameComponent.AssetCache` (`/Game/HorrorEngine/HorrorEngine.HE_SaveGameComponent` _asmaster)) (make `/Game/HorrorEngine/Blueprints/Structures/SaveStructures/AssetsSave` (`KismetSystemLibrary.GetObjectName` self) false false false false (`self.LookingCounter`) (`self.FocusingCounter`) 0 "+00000000.00:00:00.000000000" "NewEnumerator0" (struct :`Actor` "NewEnumerator0" :`MeshSettings` (struct) :`InspectionSettings` (struct :`InspectionPivotLocation` (0.0 0.0 0.0) :`Takeable` true :`InspectionAnimation` true :`InspectionAnimationSpeedSec` 0.5 :`InspectionBeginRotation` (struct) :`InspectionBeginScale` 1.0 :`MinZoomScale` 1.0 :`MaxZoomScale` 2.0 :`RotationSpeed` 2.5 :`SlideSpeed` 1.0 :`MaxSlideValue` 10.0 :`ItemName` "NSLOCTEXT(\"[E9739AD04A42D129AE2E0F8898EB0039]\", \"C253737141A6D25990F0EA89B16562DB\", \"Item Name\")" :`ItemInformation` "NSLOCTEXT(\"[E9739AD04A42D129AE2E0F8898EB0039]\", \"AAF1B837493BE118F120D1AACB5B1DCB\", \"Item Information\")" :`ReadingText` "NSLOCTEXT(\"[E9739AD04A42D129AE2E0F8898EB0039]\", \"E5EB13004502BDB01EC2589159A7B8C8\", \"Reading Text\")" :`TakeButton` (struct :`ButtonText` "NSLOCTEXT(\"[E9739AD04A42D129AE2E0F8898EB0039]\", \"D88E530E4E1FDD0D1AF1E4B60BEA0C74\", \"Take\")" :`ButtonImage` "Texture2D'\"/Game/HorrorEngine/Textures/HUD/Input_MouseLeft.Input_MouseLeft\"'") :`ExamineButton` (struct :`ButtonText` "NSLOCTEXT(\"[E9739AD04A42D129AE2E0F8898EB0039]\", \"0B0AD5A24D7D89DD08B678B6AA38057B\", \"Examine\")" :`ButtonImage` "Texture2D'\"/Game/HorrorEngine/Textures/HUD/Input_E.Input_E\"'") :`ZoomSlideButton` (struct :`ButtonText` "NSLOCTEXT(\"[E9739AD04A42D129AE2E0F8898EB0039]\", \"BDECA2694096F800123C80A0D5399C8C\", \"Zoom/Slide\")" :`ButtonImage` "Texture2D'\"/Game/HorrorEngine/Textures/HUD/Input_MouseMiddle.Input_MouseMiddle\"'") :`DismissButton` (struct :`ButtonText` "NSLOCTEXT(\"[E9739AD04A42D129AE2E0F8898EB0039]\", \"B2F06ED848685F1A84EE90B2AAAA5C86\", \"Dismiss\")" :`ButtonImage` "Texture2D'\"/Game/HorrorEngine/Textures/HUD/Input_MouseRight.Input_MouseRight\"'")) :`InventorySettings` (struct :`StorageType` "NewEnumerator3" :`NumberofItemstoAddInventory` 1 :`Interactable` true :`InteractionButton` (struct :`ButtonText` "NSLOCTEXT(\"[E9739AD04A42D129AE2E0F8898EB0039]\", \"0C85836644155E76B83859ADD6591342\", \"Use\")" :`ButtonImage` "Texture2D'\"/Game/HorrorEngine/Textures/HUD/Input_MouseLeft.Input_MouseLeft\"'") :`SwitchButton` (struct :`ButtonText` "NSLOCTEXT(\"[E9739AD04A42D129AE2E0F8898EB0039]\", \"D0E73D0E4B011D4DBB917DAC6C703EE7\", \"Switch\")" :`ButtonImage` "Texture2D'\"/Game/HorrorEngine/Textures/HUD/Input_MouseMiddle.Input_MouseMiddle\"'") :`ZoomSlideButton` (struct :`ButtonText` "NSLOCTEXT(\"[E9739AD04A42D129AE2E0F8898EB0039]\", \"A670DC0D47561CA1D4879EB3A6362628\", \"Zoom/Slide\")" :`ButtonImage` "Texture2D'\"/Game/HorrorEngine/Textures/HUD/Input_MouseRightAndMiddle.Input_MouseRightAndMiddle\"'") :`CloseInventoryButton` (struct :`ButtonText` "NSLOCTEXT(\"[E9739AD04A42D129AE2E0F8898EB0039]\", \"A7ED75C94CDAD42B395859A0CE42EB9A\", \"Close\")" :`ButtonImage` "Texture2D'\"/Game/HorrorEngine/Textures/HUD/Input_Tab.Input_Tab\"'")) :`Pistol_MeshSettingsTop` (struct) :`Vhs_CurrentTime` "+00000000.00:00:00.000000000"))))

(event `/Game/HorrorEngine/Blueprints/Core/HorrorEngineInterface.RestoreSaveData`
  (params (AssetSave :type "/Game/HorrorEngine/Blueprints/Structures/SaveStructures/AssetsSave Structure"))
  (bind (_objectname _booleanslot01 _booleanslot02 _booleanslot03 _booleanslot04 _floatslot01 _floatslot02) (break `/Game/HorrorEngine/Blueprints/Structures/SaveStructures/AssetsSave` AssetSave))
  ;[0 1 0.5572] Save Settings
  (set `self.LookingCounter` _floatslot01)
  (set `self.FocusingCounter` _floatslot02))

(fn `UserConstructionScript`
  (`/Game/HorrorEngine/Blueprints/Core/HorrorEngineMacros.HM_DefaultConstructions` (`self.CreateNewHorrorEvent`))
  (`BoxComponent.SetBoxExtent` (`self.LookTrigger`) (`self.TriggerBoxExtent`) true))