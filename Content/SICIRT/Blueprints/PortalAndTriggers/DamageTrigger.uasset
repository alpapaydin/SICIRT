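; Damage volume that repeatedly hurts the player pawn while it stays inside a box trigger.
; Begin overlap sets a burning flag, starts a self-calling delayed damage loop and runs a horror event check; end overlap clears the flag.
; The construction script applies default horror event setup, then sizes the box and offsets it by its extent so it grows from the actor origin at one corner.
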(event `self.DamageTrigger.OnComponentBeginOverlap`
  (params (OverlappedComponent :type "PrimitiveComponent Object Reference") (OtherActor :type "Actor Object Reference") (OtherComp :type "PrimitiveComponent Object Reference") (OtherBodyIndex :type Integer) (bFromSweep :type Boolean) (SweepResult :type "HitResult Structure (by ref)"))
  ;[1 1 1] Overlap Settings
  (if (== OtherActor (`GameplayStatics.GetPlayerPawn` 0))
    (set `self.Burning` true)
    (`self.BurnMF`)
    (`self.HorrorEventCheck` "NewEnumerator48")))

(event `self.DamageTrigger.OnComponentEndOverlap`
  (params (OverlappedComponent :type "PrimitiveComponent Object Reference") (OtherActor :type "Actor Object Reference") (OtherComp :type "PrimitiveComponent Object Reference") (OtherBodyIndex :type Integer))
  ;[1 1 1] Overlap Settings
  (if (== OtherActor (`GameplayStatics.GetPlayerPawn` 0))
    (set `self.Burning` false)))

(event `BurnMF`
  ;[1 1 1] Overlap Settings
  (if (`self.Burning`)
    (bind _asmaster (`/Game/HorrorEngine/Blueprints/Core/HorrorEngineFunctions.GetPlayer`))
    (`/Game/HorrorEngine/HorrorEngine.GetDamage` :`self` _asmaster :`DamagePoint` (`self.DamageValue`))
    (`KismetSystemLibrary.Delay` (`self.Get Damage Each (N) Second(s)`))
    (`self.BurnMF`)))

(fn `UserConstructionScript`
  (`/Game/HorrorEngine/Blueprints/Core/HorrorEngineMacros.HM_DefaultConstructions` (`self.CreateNewHorrorEvent`))
  (`BoxComponent.SetBoxExtent` (`self.DamageTrigger`) (`self.TriggerBoxExtent`) true)
  (`SceneComponent.K2_SetRelativeLocation` (`self.DamageTrigger`) (`self.TriggerBoxExtent`) false false))