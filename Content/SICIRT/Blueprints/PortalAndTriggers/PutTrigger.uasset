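; Placement trigger box that unlocks and fires a horror event when the required number of specific or tagged actors is inside.
; Begin and end overlaps run CalculateActors to match actors by reference or tag, then adjust Counter, ignoring overlaps during game loading.
; An exit while unlocked fires a second horror event without relocking.
; Save hooks use the player's HESaveGameComponent asset cache, with Locked and Counter restored on load.
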(event `self.PutTrigger.OnComponentBeginOverlap`
  (params (OverlappedComponent :type "PrimitiveComponent Object Reference") (OtherActor :type "Actor Object Reference") (OtherComp :type "PrimitiveComponent Object Reference") (OtherBodyIndex :type Integer) (bFromSweep :type Boolean) (SweepResult :type "HitResult Structure (by ref)"))
  ;[1 1 1] Overlap Settings
  (bind _ashe_game_instance (cast `/Game/HorrorEngine/Blueprints/Core/HE_GameInstance` (`GameplayStatics.GetGameInstance`)))
  (if (not (`/Game/HorrorEngine/Blueprints/Core/HE_GameInstance.Loading` _ashe_game_instance))
    (`self.CalculateActors` OtherActor)
    (bind _output_get (set `self.Counter` (+ (`self.Counter`) 1)))
    (if (== _output_get (+ (`KismetArrayLibrary.Array_Length` (`self.Required Actor(s) for Unlock`)) (`self.RequaredNumberOfTaggedActor(s)`)))
      (set `self.Locked` false)
      (`self.HorrorEventCheck` "NewEnumerator6"))))

(event `self.PutTrigger.OnComponentEndOverlap`
  (params (OverlappedComponent :type "PrimitiveComponent Object Reference") (OtherActor :type "Actor Object Reference") (OtherComp :type "PrimitiveComponent Object Reference") (OtherBodyIndex :type Integer))
  ;[1 1 1] Overlap Settings
  (bind _ashe_game_instance (cast `/Game/HorrorEngine/Blueprints/Core/HE_GameInstance` (`GameplayStatics.GetGameInstance`)))
  (if (not (`/Game/HorrorEngine/Blueprints/Core/HE_GameInstance.Loading` _ashe_game_instance))
    (`self.CalculateActors` OtherActor)
    (set `self.Counter` (- (`self.Counter`) 1))
    (if (not (`self.Locked`))
      (`self.HorrorEventCheck` "NewEnumerator5"))))

(event `/Game/HorrorEngine/Blueprints/Core/HorrorEngineInterface.CollectSaveData`
  ;[0 1 0.5572] Save Settings
  (bind _asmaster (`/Game/HorrorEngine/Blueprints/Core/HorrorEngineFunctions.GetPlayer`))
  (`KismetArrayLibrary.Array_Add` (`/Game/HorrorEngine/Blueprints/Core/HE_SaveGameComponent.AssetCache` (`/Game/HorrorEngine/HorrorEngine.HE_SaveGameComponent` _asmaster)) (make `/Game/HorrorEngine/Blueprints/Structures/SaveStructures/AssetsSave` (`KismetSystemLibrary.GetObjectName` self) (`self.Locked`) false false false 0.0 0.0 (`self.Counter`) "+00000000.00:00:00.000000000" "NewEnumerator0" (struct :`Actor` "NewEnumerator0" :`MeshSettings` (struct) :`InspectionSettings` (struct :`InspectionPivotLocation` (0.0 0.0 0.0) :`Takeable` true :`InspectionAnimation` true :`InspectionAnimationSpeedSec` 0.5 :`InspectionBeginRotation` (struct) :`InspectionBeginScale` 1.0 :`MinZoomScale` 1.0 :`MaxZoomScale` 2.0 :`RotationSpeed` 2.5 :`SlideSpeed` 1.0 :`MaxSlideValue` 10.0 :`ItemName` "NSLOCTEXT(\"[5C4ABA7149C69034AD3764B452A6FA51]\", \"65290FD641728D741BD3ADB295F38A9F\", \"Item Name\")" :`ItemInformation` "NSLOCTEXT(\"[5C4ABA7149C69034AD3764B452A6FA51]\", \"DE2DA431447953A18CF1B1AE8122BC06\", \"Item Information\")" :`ReadingText` "NSLOCTEXT(\"[5C4ABA7149C69034AD3764B452A6FA51]\", \"1178704345F0A2CCDA7C1599095756F6\", \"Reading Text\")" :`TakeButton` (struct :`ButtonText` "NSLOCTEXT(\"[5C4ABA7149C69034AD3764B452A6FA51]\", \"090C2A094B3F65ECB0F260A8F40FC8D3\", \"Take\")" :`ButtonImage` "Texture2D'\"/Game/HorrorEngine/Textures/HUD/Input_MouseLeft.Input_MouseLeft\"'") :`ExamineButton` (struct :`ButtonText` "NSLOCTEXT(\"[5C4ABA7149C69034AD3764B452A6FA51]\", \"B0CC4E4A437AC555E6BF73B1910220CE\", \"Examine\")" :`ButtonImage` "Texture2D'\"/Game/HorrorEngine/Textures/HUD/Input_E.Input_E\"'") :`ZoomSlideButton` (struct :`ButtonText` "NSLOCTEXT(\"[5C4ABA7149C69034AD3764B452A6FA51]\", \"4A5743874D584F179AF10DA3E6305BFC\", \"Zoom/Slide\")" :`ButtonImage` "Texture2D'\"/Game/HorrorEngine/Textures/HUD/Input_MouseMiddle.Input_MouseMiddle\"'") :`DismissButton` (struct :`ButtonText` "NSLOCTEXT(\"[5C4ABA7149C69034AD3764B452A6FA51]\", \"38EC2E9644207A9BC064B2958E778BAB\", \"Dismiss\")" :`ButtonImage` "Texture2D'\"/Game/HorrorEngine/Textures/HUD/Input_MouseRight.Input_MouseRight\"'")) :`InventorySettings` (struct :`StorageType` "NewEnumerator3" :`NumberofItemstoAddInventory` 1 :`Interactable` true :`InteractionButton` (struct :`ButtonText` "NSLOCTEXT(\"[5C4ABA7149C69034AD3764B452A6FA51]\", \"B4E3049843A29AB45E41D9A992274D98\", \"Use\")" :`ButtonImage` "Texture2D'\"/Game/HorrorEngine/Textures/HUD/Input_MouseLeft.Input_MouseLeft\"'") :`SwitchButton` (struct :`ButtonText` "NSLOCTEXT(\"[5C4ABA7149C69034AD3764B452A6FA51]\", \"C025530343DE9DA0B44D44AB3B144A78\", \"Switch\")" :`ButtonImage` "Texture2D'\"/Game/HorrorEngine/Textures/HUD/Input_MouseMiddle.Input_MouseMiddle\"'") :`ZoomSlideButton` (struct :`ButtonText` "NSLOCTEXT(\"[5C4ABA7149C69034AD3764B452A6FA51]\", \"A8873C3743B7EC878690B2887E938B93\", \"Zoom/Slide\")" :`ButtonImage` "Texture2D'\"/Game/HorrorEngine/Textures/HUD/Input_MouseRightAndMiddle.Input_MouseRightAndMiddle\"'") :`CloseInventoryButton` (struct :`ButtonText` "NSLOCTEXT(\"[5C4ABA7149C69034AD3764B452A6FA51]\", \"C6E4096840177A3718A024A08E3692AF\", \"Close\")" :`ButtonImage` "Texture2D'\"/Game/HorrorEngine/Textures/HUD/Input_Tab.Input_Tab\"'")) :`Pistol_MeshSettingsTop` (struct) :`Vhs_CurrentTime` "+00000000.00:00:00.000000000"))))

(event `/Game/HorrorEngine/Blueprints/Core/HorrorEngineInterface.RestoreSaveData`
  (params (AssetSave :type "/Game/HorrorEngine/Blueprints/Structures/SaveStructures/AssetsSave Structure"))
  (bind (_objectname _booleanslot01 _booleanslot02 _booleanslot03 _booleanslot04 _floatslot01 _floatslot02 _integerslot01) (break `/Game/HorrorEngine/Blueprints/Structures/SaveStructures/AssetsSave` AssetSave))
  ;[0 1 0.5572] Save Settings
  (set `self.Locked` _booleanslot01)
  (set `self.Counter` _integerslot01))

(fn `UserConstructionScript`
  (`/Game/HorrorEngine/Blueprints/Core/HorrorEngineMacros.HM_DefaultConstructions` (`self.CreateNewHorrorEvent`))
  (`BoxComponent.SetBoxExtent` (`self.PutTrigger`) (`self.TriggerBoxExtent`) true)
  (`SceneComponent.K2_SetRelativeLocation` (`self.PutTrigger`) (`self.TriggerBoxExtent`) false false))