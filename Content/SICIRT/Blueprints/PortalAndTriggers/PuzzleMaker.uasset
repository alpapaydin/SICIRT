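; PuzzleMaker is a counter-based puzzle gate that fires a horror event once it has been unlocked a set number of times.
; Unlock increments Counter and calls HorrorEventCheck when it exactly equals UnlockAfterNTimes, while Lock decrements it without going below zero.
; Save hooks add an asset save to the player's HESaveGameComponent cache and restore Counter from its integer slot.
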(event `self.Lock`
  (params (HorrorEvent :type Boolean))
  (bind _returnvalue (- (`self.Counter`) 1))
  (set `self.Counter` (select `bool` (<= _returnvalue 0) :`false` _returnvalue)))

(event `self.Unlock`
  (params (HorrorEvent :type Boolean))
  (bind _output_get (set `self.Counter` (+ (`self.Counter`) 1)))
  (if (== _output_get (`self.Unlock After (N) Times`))
    (`self.HorrorEventCheck` "NewEnumerator6")))

(event `/Game/HorrorEngine/Blueprints/Core/HorrorEngineInterface.CollectSaveData`
  ;[0 1 0.5572] Save Settings
  (bind _asmaster (`/Game/HorrorEngine/Blueprints/Core/HorrorEngineFunctions.GetPlayer`))
  (`KismetArrayLibrary.Array_Add` (`/Game/HorrorEngine/Blueprints/Core/HE_SaveGameComponent.AssetCache` (`/Game/HorrorEngine/HorrorEngine.HE_SaveGameComponent` _asmaster)) (make `/Game/HorrorEngine/Blueprints/Structures/SaveStructures/AssetsSave` (`KismetSystemLibrary.GetObjectName` self) false false false false 0.0 0.0 (`self.Counter`) "+00000000.00:00:00.000000000" "NewEnumerator0" (struct :`Actor` "NewEnumerator0" :`MeshSettings` (struct) :`InspectionSettings` (struct :`InspectionPivotLocation` (0.0 0.0 0.0) :`Takeable` true :`InspectionAnimation` true :`InspectionAnimationSpeedSec` 0.5 :`InspectionBeginRotation` (struct) :`InspectionBeginScale` 1.0 :`MinZoomScale` 1.0 :`MaxZoomScale` 2.0 :`RotationSpeed` 2.5 :`SlideSpeed` 1.0 :`MaxSlideValue` 10.0 :`ItemName` "NSLOCTEXT(\"[8502188645CB06B8FA9787A633A23F97]\", \"22DAE6C74C17964E4F9B2B8DBF3F8442\", \"Item Name\")" :`ItemInformation` "NSLOCTEXT(\"[8502188645CB06B8FA9787A633A23F97]\", \"2F0CED474244424C2DA969A76F0BB78B\", \"Item Information\")" :`ReadingText` "NSLOCTEXT(\"[8502188645CB06B8FA9787A633A23F97]\", \"F38E71124B0023A8CA9148BB34DA3247\", \"Reading Text\")" :`TakeButton` (struct :`ButtonText` "NSLOCTEXT(\"[8502188645CB06B8FA9787A633A23F97]\", \"3693496E486C42D4062DA3A352229D94\", \"Take\")" :`ButtonImage` "Texture2D'\"/Game/HorrorEngine/Textures/HUD/Input_MouseLeft.Input_MouseLeft\"'") :`ExamineButton` (struct :`ButtonText` "NSLOCTEXT(\"[8502188645CB06B8FA9787A633A23F97]\", \"91004C1849515BA1A6A998960CDFC8D8\", \"Examine\")" :`ButtonImage` "Texture2D'\"/Game/HorrorEngine/Textures/HUD/Input_E.Input_E\"'") :`ZoomSlideButton` (struct :`ButtonText` "NSLOCTEXT(\"[8502188645CB06B8FA9787A633A23F97]\", \"A3D8DA7D43C010781D729C8734328D61\", \"Zoom/Slide\")" :`ButtonImage` "Texture2D'\"/Game/HorrorEngine/Textures/HUD/Input_MouseMiddle.Input_MouseMiddle\"'") :`DismissButton` (struct :`ButtonText` "NSLOCTEXT(\"[8502188645CB06B8FA9787A633A23F97]\", \"3B9A306B4AE8F74F3AAC179BBEF964B7\", \"Dismiss\")" :`ButtonImage` "Texture2D'\"/Game/HorrorEngine/Textures/HUD/Input_MouseRight.Input_MouseRight\"'")) :`InventorySettings` (struct :`StorageType` "NewEnumerator3" :`NumberofItemstoAddInventory` 1 :`Interactable` true :`InteractionButton` (struct :`ButtonText` "NSLOCTEXT(\"[8502188645CB06B8FA9787A633A23F97]\", \"299E70B84ABAEB403D6650B65450E909\", \"Use\")" :`ButtonImage` "Texture2D'\"/Game/HorrorEngine/Textures/HUD/Input_MouseLeft.Input_MouseLeft\"'") :`SwitchButton` (struct :`ButtonText` "NSLOCTEXT(\"[8502188645CB06B8FA9787A633A23F97]\", \"D27AD0D14CB167C636D678B895A99BB3\", \"Switch\")" :`ButtonImage` "Texture2D'\"/Game/HorrorEngine/Textures/HUD/Input_MouseMiddle.Input_MouseMiddle\"'") :`ZoomSlideButton` (struct :`ButtonText` "NSLOCTEXT(\"[8502188645CB06B8FA9787A633A23F97]\", \"B92F81F8417E9DB897ED5DB88B352821\", \"Zoom/Slide\")" :`ButtonImage` "Texture2D'\"/Game/HorrorEngine/Textures/HUD/Input_MouseRightAndMiddle.Input_MouseRightAndMiddle\"'") :`CloseInventoryButton` (struct :`ButtonText` "NSLOCTEXT(\"[8502188645CB06B8FA9787A633A23F97]\", \"C1E1D8CC4CBA5780E89CB3B7D62DF2BB\", \"Close\")" :`ButtonImage` "Texture2D'\"/Game/HorrorEngine/Textures/HUD/Input_Tab.Input_Tab\"'")) :`Pistol_MeshSettingsTop` (struct) :`Vhs_CurrentTime` "+00000000.00:00:00.000000000"))))

(event `/Game/HorrorEngine/Blueprints/Core/HorrorEngineInterface.RestoreSaveData`
  (params (AssetSave :type "/Game/HorrorEngine/Blueprints/Structures/SaveStructures/AssetsSave Structure"))
  ;[0 1 0.5572] Save Settings
  (set `self.Counter` (`.IntegerSlot01_75_ABA8053D4F033D11B1D4ECB38D77F6AB` (break `/Game/HorrorEngine/Blueprints/Structures/SaveStructures/AssetsSave` AssetSave))))

(fn `UserConstructionScript`
  (`parent.UserConstructionScript`)
  (`/Game/HorrorEngine/Blueprints/Core/HorrorEngineMacros.HM_DefaultConstructions` (`self.CreateNewHorrorEvent`)))