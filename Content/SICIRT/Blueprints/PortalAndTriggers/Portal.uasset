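; Horror-game portal that teleports on Use or on overlap gated by a B_Kanka cast, with sound, particles and optional fading post-process effects.
; The TeleportLocationVision capture feeds a render target into the portal's dynamic materials and marks the normal destination.
; Lock and Unlock switch the destination between TrapLocation and that point, firing horror events.
; Timeline rotation and looping-style ambience start at BeginPlay, and save hooks handle the lock state.
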(event `self.ReceiveBeginPlay`
  ;[1 1 1] BeginPlay Settings
  (`self.CreateRenderTarget`)
  (`self.SetPlayer`)
  (`self.SelectTeleportLocation`)
  (`self.PortalTurnAnimation`)
  (`self.PortalTurnSound`))

(event `PortalTeleportEffect`
  ;[1 1 1] Teleport Effect Settings
  (`/Game/HorrorEngine/Blueprints/Core/HorrorEngineMacros.HM_3DSound` null false (`self.TeleportSound`) (`self.Portal`) (`self.PortalAttenuation`))
  (`GameplayStatics.SpawnEmitterAttached` (`self.TeleportParticleEffect`) (`self.Portal`) "None" (0.0 0.0 0.0) (struct) (1.0 1.0 1.0) "SnapToTarget"))

(event `SetPlayer`
  ;[1 1 1] BeginPlay Settings
)

(event `SelectTeleportLocation`
  ;[1 1 1] BeginPlay Settings
  (if (`self.Locked (TeleportsToTrapLocation)`)
    (set `self.SelectedLocation` (`SceneComponent.K2_GetComponentLocation` (`self.TrapLocation`)))
    (else
      (set `self.SelectedLocation` (`SceneComponent.K2_GetComponentLocation` (`self.TeleportLocationVision`))))))

(event `ComponentTeleportEffect`
  (params (AttachToComponent :type "SceneComponent Object Reference"))
  ;[1 1 1] Teleport Effect Settings
  (`/Game/HorrorEngine/Blueprints/Core/HorrorEngineMacros.HM_3DSound` null false (`self.TeleportSound`) AttachToComponent (`self.PortalAttenuation`))
  (`GameplayStatics.SpawnEmitterAttached` (`self.TeleportParticleEffect`) AttachToComponent "None" (0.0 0.0 0.0) (struct) (1.0 1.0 1.0) "SnapToTarget"))

(event `PortalTurnAnimation`
  ;[1 1 1] BeginPlay Settings
  (bind (_direction _animation) (`Timeline|PortalRotationTimeline`)
    (:`Update`
      (`SceneComponent.K2_SetRelativeRotation` (`self.Portal`) (`KismetMathLibrary.MakeRotator` _animation _animation _animation) false false)
      (`SceneComponent.K2_SetRelativeRotation` (`self.PortalAdd3`) (`KismetMathLibrary.MakeRotator` 0.0 0.0 _animation) false false))))

(event `PlayerTeleportEffect`
  ;[1 1 1] Teleport Effect Settings
  (`GameplayStatics.SpawnSound2D` (`self.TeleportSound`) 1.0 1.0 0.0 null)
  (bind _asmaster (`/Game/HorrorEngine/Blueprints/Core/HorrorEngineFunctions.GetPlayer`))
  (`GameplayStatics.SpawnEmitterAttached` (`self.TeleportParticleEffect`) (`/Game/HorrorEngine/HorrorEngine.PlayerCamera` _asmaster) "None" (35.0 0.0 0.0) (struct) (1.0 1.0 1.0) "SnapToTarget")
  (`self.HorrorEventCheck` "NewEnumerator27"))

(event `PortalTurnSound`
  ;[1 1 1] BeginPlay Settings
  (`/Game/HorrorEngine/Blueprints/Core/HorrorEngineMacros.HM_3DSound` null false (`self.PortalSound`) (`self.Portal`) (`self.PortalAttenuation`))
  (`/Game/HorrorEngine/Blueprints/Core/HorrorEngineMacros.HM_3DSound` null false (`self.PortalNearSound`) (`self.Portal`) (`self.PortalNearAttenuation`)))

(event `TeleportedAreaEffect`
  ;[1 1 1] Teleport Effect Settings
  (if (`self.TeleportVisualEffect`)
    (set `PostProcessComponent.bEnabled` true (`self.TeleportPostProcess`))
    (set `PostProcessComponent.bEnabled` true (`self.TrapPostProcess`))
    (bind (_direction _animation) (`Timeline|EffectFadeOutTimeline` :!via `PlayFromStart`)
      (:`Update`
        (bind _output_get (set `PostProcessComponent.BlendWeight` _animation (`self.TeleportPostProcess`)))
        (set `PostProcessComponent.BlendWeight` _output_get (`self.TrapPostProcess`)))
      (:`Finished`
        (set `PostProcessComponent.bEnabled` false (`self.TeleportPostProcess`))
        (set `PostProcessComponent.bEnabled` false (`self.TrapPostProcess`))))))

(event `self.Use`
  (params (HorrorEvent :type Boolean))
  ;[1 1 1] Interaction Settings
  (`SceneComponent.K2_SetWorldLocation` (`self.Player`) (`self.SelectedLocation`) false false)
  (`self.PlayerTeleportEffect`)
  (`self.TeleportedAreaEffect`))

(event `self.Collision.OnComponentBeginOverlap`
  (params (OverlappedComponent :type "PrimitiveComponent Object Reference") (OtherActor :type "Actor Object Reference") (OtherComp :type "PrimitiveComponent Object Reference") (OtherBodyIndex :type Integer) (bFromSweep :type Boolean) (SweepResult :type "HitResult Structure (by ref)"))
  ;[1 1 1] Interaction Settings
  (bind _asb_kanka (cast `/Game/SICIRT/Blueprints/Characters/Kanka/B_Kanka` OtherComp))
  (set `self.Player` (`Character.CapsuleComponent` _asb_kanka))
  (`SceneComponent.K2_SetWorldLocation` OtherComp (`self.SelectedLocation`) false false)
  (if (== (`self.Player`) OtherComp)
    (`self.PlayerTeleportEffect`)
    (`self.TeleportedAreaEffect`)
    (`self.PortalTeleportEffect`)
    (else
      (`self.ComponentTeleportEffect` OtherComp)
      (`self.TeleportedAreaEffect`)
      (`self.PortalTeleportEffect`)
      (bind _asmaster (`/Game/HorrorEngine/Blueprints/Core/HorrorEngineFunctions.GetPlayer`))
      (bind _heldingref (`/Game/HorrorEngine/HorrorEngine.HeldingRef` _asmaster))
      (if (== _heldingref OtherActor)
        (`/Game/HorrorEngine/Blueprints/Core/PhysicsObject.ReleaseObject` _heldingref)))))

(event `self.Lock`
  (params (HorrorEvent :type Boolean))
  ;[1 1 1] Interaction Settings
  (set `self.Locked (TeleportsToTrapLocation)` true)
  (`self.SelectTeleportLocation`)
  (`self.HorrorEventCheck` "NewEnumerator5"))

(event `self.Unlock`
  (params (HorrorEvent :type Boolean))
  ;[1 1 1] Interaction Settings
  (set `self.Locked (TeleportsToTrapLocation)` false)
  (`self.SelectTeleportLocation`)
  (`self.HorrorEventCheck` "NewEnumerator6"))

(event `self.Shoot`
  (params (HorrorEvent :type Boolean))
  ;[1 1 1] Interaction Settings
  (`self.PortalTeleportEffect`))

(event `/Game/HorrorEngine/Blueprints/Core/HorrorEngineInterface.CollectSaveData`
  ;[0 1 0.5572] Save Settings
  (bind _asmaster (`/Game/HorrorEngine/Blueprints/Core/HorrorEngineFunctions.GetPlayer`))
  (`KismetArrayLibrary.Array_Add` (`/Game/HorrorEngine/Blueprints/Core/HE_SaveGameComponent.AssetCache` (`/Game/HorrorEngine/HorrorEngine.HE_SaveGameComponent` _asmaster)) (make `/Game/HorrorEngine/Blueprints/Structures/SaveStructures/AssetsSave` (`KismetSystemLibrary.GetObjectName` self) (`self.Locked (TeleportsToTrapLocation)`) false false false 0.0 0.0 0 "+00000000.00:00:00.000000000" "NewEnumerator0" (struct :`Actor` "NewEnumerator0" :`MeshSettings` (struct) :`InspectionSettings` (struct :`InspectionPivotLocation` (0.0 0.0 0.0) :`Takeable` true :`InspectionAnimation` true :`InspectionAnimationSpeedSec` 0.5 :`InspectionBeginRotation` (struct) :`InspectionBeginScale` 1.0 :`MinZoomScale` 1.0 :`MaxZoomScale` 2.0 :`RotationSpeed` 2.5 :`SlideSpeed` 1.0 :`MaxSlideValue` 10.0 :`ItemName` "NSLOCTEXT(\"[ED9D9A64409C1CCC61C49DBAF716840E]\", \"41C1E6414FA651B2F62A1596657249DC\", \"Item Name\")" :`ItemInformation` "NSLOCTEXT(\"[ED9D9A64409C1CCC61C49DBAF716840E]\", \"E9B49E504329FEC4258E1F9A85786738\", \"Item Information\")" :`ReadingText` "NSLOCTEXT(\"[ED9D9A64409C1CCC61C49DBAF716840E]\", \"CAFF248F407AC296B7AED783C352D3C5\", \"Reading Text\")" :`TakeButton` (struct :`ButtonText` "NSLOCTEXT(\"[ED9D9A64409C1CCC61C49DBAF716840E]\", \"8C3EBFA14824AD6601F37B90DE7893F8\", \"Take\")" :`ButtonImage` "Texture2D'\"/Game/HorrorEngine/Textures/HUD/Input_MouseLeft.Input_MouseLeft\"'") :`ExamineButton` (struct :`ButtonText` "NSLOCTEXT(\"[ED9D9A64409C1CCC61C49DBAF716840E]\", \"0AF3052F4B89D8A8DB002ABB64E42C05\", \"Examine\")" :`ButtonImage` "Texture2D'\"/Game/HorrorEngine/Textures/HUD/Input_E.Input_E\"'") :`ZoomSlideButton` (struct :`ButtonText` "NSLOCTEXT(\"[ED9D9A64409C1CCC61C49DBAF716840E]\", \"7973B2BD470BEB76100591B88B6EAB8D\", \"Zoom/Slide\")" :`ButtonImage` "Texture2D'\"/Game/HorrorEngine/Textures/HUD/Input_MouseMiddle.Input_MouseMiddle\"'") :`DismissButton` (struct :`ButtonText` "NSLOCTEXT(\"[ED9D9A64409C1CCC61C49DBAF716840E]\", \"6E6F12BC46B96918B69DD797F801256F\", \"Dismiss\")" :`ButtonImage` "Texture2D'\"/Game/HorrorEngine/Textures/HUD/Input_MouseRight.Input_MouseRight\"'")) :`InventorySettings` (struct :`StorageType` "NewEnumerator3" :`NumberofItemstoAddInventory` 1 :`Interactable` true :`InteractionButton` (struct :`ButtonText` "NSLOCTEXT(\"[ED9D9A64409C1CCC61C49DBAF716840E]\", \"7E02F8B64B4282BB41B89991CC7386BF\", \"Use\")" :`ButtonImage` "Texture2D'\"/Game/HorrorEngine/Textures/HUD/Input_MouseLeft.Input_MouseLeft\"'") :`SwitchButton` (struct :`ButtonText` "NSLOCTEXT(\"[ED9D9A64409C1CCC61C49DBAF716840E]\", \"E95CA25B4E493DBC5F3E2C92EE280261\", \"Switch\")" :`ButtonImage` "Texture2D'\"/Game/HorrorEngine/Textures/HUD/Input_MouseMiddle.Input_MouseMiddle\"'") :`ZoomSlideButton` (struct :`ButtonText` "NSLOCTEXT(\"[ED9D9A64409C1CCC61C49DBAF716840E]\", \"0FCEEFB14219ADD328A2919D94756D33\", \"Zoom/Slide\")" :`ButtonImage` "Texture2D'\"/Game/HorrorEngine/Textures/HUD/Input_MouseRightAndMiddle.Input_MouseRightAndMiddle\"'") :`CloseInventoryButton` (struct :`ButtonText` "NSLOCTEXT(\"[ED9D9A64409C1CCC61C49DBAF716840E]\", \"7ADAF53E4DD3E5A9B35CB3A7C3CC3D00\", \"Close\")" :`ButtonImage` "Texture2D'\"/Game/HorrorEngine/Textures/HUD/Input_Tab.Input_Tab\"'")) :`Pistol_MeshSettingsTop` (struct) :`Vhs_CurrentTime` "+00000000.00:00:00.000000000"))))

(event `/Game/HorrorEngine/Blueprints/Core/HorrorEngineInterface.RestoreSaveData`
  (params (AssetSave :type "/Game/HorrorEngine/Blueprints/Structures/SaveStructures/AssetsSave Structure"))
  ;[0 1 0.5572] Save Settings
  (set `self.Locked (TeleportsToTrapLocation)` (`.BooleanSlot01_63_ED79FB5D49E9ED6768D7AE96EDFDE8DB` (break `/Game/HorrorEngine/Blueprints/Structures/SaveStructures/AssetsSave` AssetSave))))

(fn `CreateRenderTarget`
  (bind _returnvalue (`KismetRenderingLibrary.CreateRenderTarget2D` 256))
  (bind _output_get (set `SceneCaptureComponent2D.TextureTarget` _returnvalue (`self.TeleportLocationVision`)))
  (bind _returnvalue_2 (`PrimitiveComponent.CreateDynamicMaterialInstance` (`self.Portal`) 0 "/Game/HorrorEngine/Materials/HE_Portal.HE_Portal" "None"))
  (`MaterialInstanceDynamic.SetTextureParameterValue` _returnvalue_2 "PortalCapture" _output_get)
  (bind _returnvalue_3 (`PrimitiveComponent.CreateDynamicMaterialInstance` (`self.PortalAdd3`) 0 "/Game/HorrorEngine/Materials/HE_PortalAdd3.HE_PortalAdd3" "None"))
  (`MaterialInstanceDynamic.SetTextureParameterValue` _returnvalue_3 "PortalCapture" _output_get))

(fn `UserConstructionScript`
  (`/Game/HorrorEngine/Blueprints/Core/HorrorEngineMacros.HM_DefaultConstructions` (`self.CreateNewHorrorEvent`))
  (`self.CreateRenderTarget`))