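; PhotoTrigger is a box trigger actor that supplies the content of a photo taken with the player's Cameroid.
; Its TakePhoto event copies the configured horror events, developed photo name and information, and non-dismissable story item setting onto the player's CameroidPhoto.
; The construction script runs shared HM default constructions and sizes the box from an exposed extent.
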(event `self.TakePhoto`
  ;[1 1 1] Take Photo Settings
  (bind _asmaster (`/Game/HorrorEngine/Blueprints/Core/HorrorEngineFunctions.GetPlayer`))
  (bind _cameroidphoto (`/Game/HorrorEngine/HorrorEngine.CameroidPhoto` _asmaster))
  (set `/Game/HorrorEngine/Blueprints/Core/Use.HorrorEvents` (`self.CreateNewHorrorEvent (for Photo)`) _cameroidphoto)
  (set `/Game/HorrorEngine/Blueprints/UsableAssets/Inventory/CameroidPhotoDeveloped.DevelopedPhotoInfo` (`self.DevelopedPhotoName`) _cameroidphoto)
  (set `/Game/HorrorEngine/Blueprints/UsableAssets/Inventory/CameroidPhotoDeveloped.DevelopedPhotoInformation` (`self.DevelopedPhotoInformation`) _cameroidphoto)
  (set `/Game/HorrorEngine/Blueprints/UsableAssets/Inventory/CameroidPhotoStatic.StoryItem` (`self.StoryItem(CanNotDismiss)`) _cameroidphoto))

(fn `UserConstructionScript`
  (`/Game/HorrorEngine/Blueprints/Core/HorrorEngineMacros.HM_DefaultConstructions` (`self.CreateNewHorrorEvent`))
  (`BoxComponent.SetBoxExtent` (`self.PhotoTrigger`) (`self.TriggerBoxExtent`) true))