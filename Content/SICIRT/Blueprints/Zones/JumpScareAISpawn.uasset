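; Jump scare trigger zone that spawns a scare AI when the B_Kanka player character overlaps it.
; The AI (B_JumpScareAI running BT_JumpScare) spawns at the character's JumpScareArrow component.
; Döndür then snaps the character's control rotation from its head socket toward the AI's head, and an alarm sound plays.
; A flag and delay form a short cooldown against retriggering.
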(event `Döndür`
  (`Controller.SetControlRotation` (`Pawn.GetController` (`self.As B Kanka`)) (`KismetMathLibrary.FindLookAtRotation` (`SceneComponent.GetSocketLocation` (`Character.Mesh` (`self.As B Kanka`)) "Head") (`SceneComponent.GetSocketLocation` (`Character.Mesh` (stale `self.ReceiveActorBeginOverlap` _output_get_3)) "Head"))))

(event `self.ReceiveActorBeginOverlap`
  (params (OtherActor :type "Actor Object Reference"))
  (bind _output_get (set `self.OverlapActor` OtherActor))
  (`KismetSystemLibrary.PrintString` (`KismetSystemLibrary.GetDisplayName` _output_get))
  (if (not (`self.onCooldown`))
    (if (== (`GameplayStatics.GetObjectClass` (`self.OverlapActor`)) "/Game/SICIRT/Blueprints/Characters/Kanka/B_Kanka.B_Kanka_C")
      (bind _asb_kanka (cast `/Game/SICIRT/Blueprints/Characters/Kanka/B_Kanka` (`self.OverlapActor`)))
      (bind _output_get_2 (set `self.As B Kanka` _asb_kanka))
      (bind (_returnvalue_location _returnvalue_rotation) (`KismetMathLibrary.BreakTransform` (`SceneComponent.K2_GetComponentToWorld` (`/Game/SICIRT/Blueprints/Characters/Kanka/B_Kanka.JumpScareArrow` _output_get_2))))
      (bind _returnvalue (`AIBlueprintHelperLibrary.SpawnAIFromClass` "/Game/SICIRT/Blueprints/Foes/JumpScareAI/B_JumpScareAI.B_JumpScareAI_C" "/Game/SICIRT/Blueprints/Foes/JumpScareAI/BT_JumpScare.BT_JumpScare" _returnvalue_location _returnvalue_rotation true null))
      (bind _asb_jump_scare_ai (cast `/Game/SICIRT/Blueprints/Foes/JumpScareAI/B_JumpScareAI` _returnvalue))
      (bind _output_get_3 (set `self.AICar` _asb_jump_scare_ai))
      (`self.Döndür`)
      ;[1 1 1] korkunç bi ses bi de bundan sonra korkunç bi foto bumm
      (`GameplayStatics.PlaySound2D` "/Game/SICIRT/Assets/_Audios/Environment/Alarm_Cue.Alarm_Cue" 0.01 1.0 0.0 null null)
      (set `self.onCooldown` true)
      (`KismetSystemLibrary.Delay` 5.0)
      (set `self.onCooldown` false))))

(fn `UserConstructionScript`)