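; B_KankaYapıcı is an overlap-triggered actor that turns a B_GM into a B_Kanka.
; When a B_GM overlaps it, it spawns a B_Kanka at the transform of the PlayerStart returned by GetActorOfClass.
; The B_GM's owning B_GMKontroller then possesses the new B_Kanka and the B_GM is destroyed.
; The owner cast follows the spawn, so a failed cast leaves both actors in the world.
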(event `self.ReceiveActorBeginOverlap`
  (params (OtherActor :type "Actor Object Reference"))
  (bind _asb_gm (cast `/Game/SICIRT/Blueprints/Characters/GM/B_GM` OtherActor))
  (set `self.As B GM` _asb_gm)
  (bind _returnvalue (`|SpawnActorFromClass` "/Game/SICIRT/Blueprints/Characters/Kanka/B_Kanka.B_Kanka_C" (`self.Get Player Start Transform`) "Undefined" "OverrideRootScale" null null))
  (bind _asb_gmkontroller (cast `/Game/SICIRT/Blueprints/Characters/GM/B_GMKontroller` (`self.GetOwner` (`self.As B GM`))))
  (`Controller.Possess` _asb_gmkontroller _returnvalue)
  (`self.K2_DestroyActor` (`self.As B GM`)))

(fn `Get Player Start Transform`
  (returns (ReturnValue :type "Transform Structure (by ref)"))
  (bind _returnvalue (`GameplayStatics.GetActorOfClass` "/Script/Engine.PlayerStart"))
  (return (`self.GetTransform` _returnvalue)))

(fn `UserConstructionScript`)